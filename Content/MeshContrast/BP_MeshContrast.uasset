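; BP_MeshContrast is an actor that shows static or skeletal meshes and switches them between normal and wireframe views.
; AddMeshComponents spawns two components per supplied mesh at runtime, a visible original and a hidden wireframe twin, in parallel arrays.
; SetWireframeMaterial applies the Wireframe material to the twins, though on static meshes it only sets slot 0.
; ToggleWireMode swaps visibility between each pair by array index, avoiding material swaps when toggling.
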(event Custom|SetWireframeMaterial
  (Utilities|FlowControl|Sequence
    (:then_0
      (for _array_element (Variables|Default|GetSKMComponents_wire)
        (for _index (range 0 (- (Utilities|Array|Length (Rendering|Material|GetMaterials _array_element)) 1))
          (Rendering|Material|SetMaterial _array_element _index "/Game/MeshContrast/Wireframe.Wireframe"))))
    (:then_1
      (for _array_element_2 (Variables|Default|GetSMComponents_wire)
        (for _index_2 (range 0 (- (Utilities|Array|Length (Rendering|Material|GetMaterials _array_element_2)) 1))
          (Rendering|Material|SetMaterial _array_element_2 0 "/Game/MeshContrast/Wireframe.Wireframe"))))))

(event Custom|ToggleWireMode
  (params (wire :type Boolean))
  (if wire
    (Utilities|FlowControl|Sequence
      (:then_0
        (for (_array_element _array_index) (Variables|Default|GetSKMComponents)
          (Rendering|SetVisibility _array_element false false)
          (Rendering|SetVisibility (Utilities|Array|Get(acopy) (Variables|Default|GetSKMComponents_wire) _array_index) true false)))
      (:then_1
        (for (_array_element_2 _array_index_2) (Variables|Default|GetSMComponents)
          (Rendering|SetVisibility _array_element_2 false false)
          (Rendering|SetVisibility (Utilities|Array|Get(acopy) (Variables|Default|GetSMComponents_wire) _array_index_2) true false))))
    (else
      (Utilities|FlowControl|Sequence
        (:then_0
          (for (_array_element_3 _array_index_3) (Variables|Default|GetSKMComponents)
            (Rendering|SetVisibility _array_element_3 true false)
            (Rendering|SetVisibility (Utilities|Array|Get(acopy) (Variables|Default|GetSKMComponents_wire) _array_index_3) false false)))
        (:then_1
          (for (_array_element_4 _array_index_4) (Variables|Default|GetSMComponents)
            (Rendering|SetVisibility _array_element_4 true false)
            (Rendering|SetVisibility (Utilities|Array|Get(acopy) (Variables|Default|GetSMComponents_wire) _array_index_4) false false)))))))

(event Custom|AddMeshComponents
  (params (SM%20or%20SKM :type Boolean) (Mesh :type Array%20of%20Object%20Object%20References))
  (if SM%20or%20SKM
    (for _array_element Mesh
      (bind _asstatic_mesh (Utilities|Casting|CastToStaticMesh _array_element))
      ;[0.15 0.15 0.15 0.5] Comment
      (bind _returnvalue (AddComponent|AddStaticMeshComponent false))
      (Components|StaticMesh|SetStaticMesh _returnvalue _asstatic_mesh)
      (Utilities|Array|AddUnique (Variables|Default|GetSMComponents) _returnvalue)
      ;[0.15 0.15 0.15 0.5] Comment
      (bind _returnvalue_2 (AddComponent|AddStaticMeshComponent false))
      (Components|StaticMesh|SetStaticMesh _returnvalue_2 _asstatic_mesh)
      (Utilities|Array|AddUnique (Variables|Default|GetSMComponents_wire) _returnvalue_2)
      (Rendering|SetVisibility _returnvalue_2 false false))
    (else
      (for _array_element_2 Mesh
        (bind _asskeletal_mesh (Utilities|Casting|CastToSkeletalMesh _array_element_2))
        ;[0.15 0.15 0.15 0.5] Comment
        (bind _returnvalue_3 (AddComponent|AddSkeletalMeshComponent false))
        (Components|SkeletalMesh|SetSkeletalMeshAsset _returnvalue_3 _asskeletal_mesh)
        (Utilities|Array|AddUnique (Variables|Default|GetSKMComponents) _returnvalue_3)
        ;[0.15 0.15 0.15 0.5] Comment
        (bind _returnvalue_4 (AddComponent|AddSkeletalMeshComponent false))
        (Components|SkeletalMesh|SetSkeletalMeshAsset _returnvalue_4 _asskeletal_mesh)
        (Utilities|Array|AddUnique (Variables|Default|GetSKMComponents_wire) _returnvalue_4)
        (Rendering|SetVisibility _returnvalue_4 false false)))))

(event EventBeginPlay)

(event Collision|EventActorBeginOverlap
  (params (OtherActor :type Actor%20Object%20Reference)))

(event EventTick
  (params (DeltaSeconds :type Float%20%28single-precision%29)))

(fn ConstructionScript)